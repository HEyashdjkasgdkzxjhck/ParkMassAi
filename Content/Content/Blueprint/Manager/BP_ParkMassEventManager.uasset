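; BP_ParkMassEventManager spawns person alerts at area-tagged points in the level and shows a matching popup.
; On BeginPlay it caches all BP_MassSpawnPoint actors, which are looked up by AreaID.
; TriggerPersonAlert optionally clears prior alerts, spawns and titles a BP_AlertPersonActor at the matching point, then opens a WBP_AlertPopup with title and description.
; ClearActiveAlerts destroys every tracked alert actor and removes only the most recently created popup.
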(event EventBeginPlay
  (bind _outactors (Actor|GetAllActorsOfClass "/ParkMassAI/Content/Blueprint/SpawnPoint/BP_MassSpawnPoint.BP_MassSpawnPoint_C"))
  (Variables|Default|SetSpawnPoints _outactors))

(event Collision|EventActorBeginOverlap
  (params (OtherActor :type Actor%20Object%20Reference)))

(event EventTick
  (params (DeltaSeconds :type Float%20%28single-precision%29)))

(fn ConstructionScript)

(fn FindSpawnPointbyAreaID
  (params (InAreaID :type Name))
  (bind _array_element (Utilities|Array|ForEachLoopwithBreak (Variables|Default|GetSpawnPoints))
    (:LoopBody
      (if (== InAreaID (Variables|/ParkMassAI/Content/Blueprint/SpawnPoint/BP_MassSpawnPoint.BP_MassSpawnPoint_C|GetAreaID _array_element))
        (return _array_element (== InAreaID (Variables|/ParkMassAI/Content/Blueprint/SpawnPoint/BP_MassSpawnPoint.BP_MassSpawnPoint_C|GetAreaID _array_element)))))
    (:Completed
      (return 0 false))))

(fn TriggerPersonAlert
  (params (InAreaId :type Name) (AlertTitle :type Text) (AlertDesc :type Text) (bClearPreviousAlert :type Boolean))
  (if bClearPreviousAlert
    (CallFunction|ClearActiveAlerts))
  (bind (_foundpoint _bfound) (CallFunction|FindSpawnPointbyAreaID InAreaId))
  (if _bfound
    (bind _spawntransform (Default|GetSpawnTransform _foundpoint))
    (bind _returnvalue (Game|SpawnActorfromClass (Variables|Default|GetAlertPersonClass) _spawntransform "AlwaysSpawn" "MultiplyWithRoot" 0 0))
    (bind _asbp_alert_person_actor (Utilities|Casting|CastToBP_AlertPersonActor _returnvalue))
    (Default|InitAlertPerson _asbp_alert_person_actor AlertTitle)
    (bind _output_get (Variables|Default|SetLastSpawnedActor _returnvalue))
    (Utilities|Array|Add (Variables|Default|GetActiveAlertActors) _output_get)
    (bind _returnvalue_2 (UserInterface|CreateWidget (Variables|Default|GetAlertPopupClass) (Game|GetPlayerController 0)))
    (bind _output_get_2 (Variables|Default|SetCurrentAlertWidget _returnvalue_2))
    (bind _aswbp_alert_popup (Utilities|Casting|CastToWBP_AlertPopup _output_get_2))
    (Default|InitAlertPopup _aswbp_alert_popup AlertTitle AlertDesc)
    (UserInterface|Viewport|AddtoViewport _aswbp_alert_popup 0)
    (else
      (Development|PrintString "Print String 提示找不到 SpawnPoint"))))

(fn ClearActiveAlerts
  (Utilities|FlowControl|Sequence
    (:then_0
      (for _array_element (Variables|Default|GetActiveAlertActors)
        (Utilities|IsValid _array_element
          (:Is%20Valid
            (Actor|DestroyActor _array_element))))
      (Utilities|Array|Clear (Variables|Default|GetActiveAlertActors)))
    (:then_1
      (Utilities|IsValid (Variables|Default|GetCurrentAlertWidget)
        (:Is%20Valid
          (Widget|RemovefromParent (Variables|Default|GetCurrentAlertWidget))
          (Variables|Default|SetCurrentAlertWidget 0)
          (Variables|Default|SetLastSpawnedActor 0))))))