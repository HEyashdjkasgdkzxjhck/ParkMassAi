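; BP_NormalPersonActor is a character actor under MassAI that adds a simple procedural idle sway to its skeletal mesh.
; BeginPlay caches the mesh's initial relative location and picks a random phase within one sine cycle.
; While EnableIdleMotion is set, Tick offsets the mesh along local X with a time-based sine scaled by speed and amount, so instances move out of sync.
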(event EventBeginPlay
  (Variables|Default|SetInitialMeshLocation (Variables|/Script/Engine.SceneComponent|GetRelativeLocation (Variables|Default|GetSkeletalMesh)))
  (Variables|Default|SetRandomPhase (Math|Random|RandomFloatinRange 0.0 6.28)))

(event Collision|EventActorBeginOverlap
  (params (OtherActor :type Actor%20Object%20Reference)))

(event EventTick
  (params (DeltaSeconds :type Float%20%28single-precision%29))
  (if (Variables|Default|GetbEnableIdleMotion)
    (Transformation|SetRelativeLocation (Variables|Default|GetSkeletalMesh) (+ (Variables|Default|GetInitialMeshLocation) (Math|Vector|MakeVector (* (Math|Trig|Sin(Radians) (+ (* (Utilities|Time|GetGameTimeinSeconds) (Variables|Default|GetIdleMotionSpeed)) (Variables|Default|GetRandomPhase))) (Variables|Default|GetIdleMotionAmount)) 0.0 0.0)) false false)))

(fn ConstructionScript)