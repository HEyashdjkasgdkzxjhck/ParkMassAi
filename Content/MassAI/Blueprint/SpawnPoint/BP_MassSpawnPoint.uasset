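; BP_MassSpawnPoint is a placeable spawn point that supplies a transform, apparently for Mass AI spawning, as its name and folder suggest.
; GetSpawnTransform returns the actor's location, optionally offset horizontally by a random unit vector's X and Y scaled by SpawnRadius when UseRandomRadius is set.
; Rotation comes from the Arrow component and scale stays at one.
; The event graph and construction script contain no active logic.
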(event EventBeginPlay)

(event Collision|EventActorBeginOverlap
  (params (OtherActor :type Actor%20Object%20Reference)))

(event EventTick
  (params (DeltaSeconds :type Float%20%28single-precision%29)))

(fn ConstructionScript)

(fn GetSpawnTransform
  (bind _returnvalue (Math|Random|RandomUnitVector))
  (bind (_x _y) (Math|Vector|BreakVector _returnvalue))
  (if (Variables|Default|GetbUseRandomRadius)
    (return (Math|Transform|MakeTransform (+ (Transformation|GetActorLocation) (* (Math|Vector|MakeVector _x _y 0.0) (Variables|Default|GetSpawnRadius))) (Transformation|GetWorldRotation (Variables|Default|GetArrow))))
    (else
      (return (Math|Transform|MakeTransform (Transformation|GetActorLocation) (Transformation|GetWorldRotation (Variables|Default|GetArrow)))))))